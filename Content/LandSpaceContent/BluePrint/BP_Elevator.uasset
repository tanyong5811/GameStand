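; Elevator actor that travels vertically between stored level locations and reports its movement, floor number and power state through BP_GameMode1 dispatchers.
; StartTeleport lights the lamp, sets directional Niagara, closes any open door, then lets Tick interpolate height at constant speed, cue a sound near arrival and reopen on arrival.
; The floor number mesh follows actor height.
; StopTeleport halts movement, flickers light, number and particles on a looping timer, then cuts them.
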(event `StopTeleport`
  (bind _audio1 (`self.Audio1`))
  (set `self.Start` false)
  (`ActorComponent.SetActive` _audio1 true true)
  (`AudioComponent.Play` _audio1 0.0)
  (`/Game/ALocalContent/Blueprint/BP_GameMode1.OnDispatchLevelStartFix` (`self.As BP Game Mode 1`))
  (bind _returnvalue (`KismetSystemLibrary.K2_SetTimerDelegate` (delegate `CustomEvent_0`) (`GameplayStatics.GetWorldDeltaSeconds`) true))
  (`KismetSystemLibrary.Delay` 2.2)
  (`KismetSystemLibrary.K2_ClearAndInvalidateTimerHandle` _returnvalue)
  (`LightComponent.SetIntensity` (`self.PointLight`) 0.0)
  (`MaterialInstanceDynamic.SetVectorParameterValue` (`self.Material`) "color" (`self.Close`))
  (`StaticMeshComponent.SetStaticMesh` (`self.Number`) null)
  (`self.ShowNiagaraxiajian` 0.0)
  (`/Game/ALocalContent/Blueprint/BP_GameMode1.OnDispatchLevelBatteryState` (`self.As BP Game Mode 1`) false))

(event `CustomEvent_0`
  (`LightComponent.SetIntensity` (`self.PointLight`) (`KismetMathLibrary.RandomFloatInRange` 1.0 3000.0))
  (bind _output_get (set `self.NewVar_0` (`KismetMathLibrary.RandomBool`)))
  (`/Game/ALocalContent/Blueprint/BP_GameMode1.OnDispatchLevelBatteryState` (`self.As BP Game Mode 1`) _output_get)
  (if _output_get
    (`self.ShowElevatorNumber`)
    (`self.ShowNiagaraxiajian` 1.5 (`self.IsTop`))
    (else
      (`StaticMeshComponent.SetStaticMesh` (`self.Number`) null)
      (`self.ShowNiagaraxiajian` 0.0))))

(event `self.ReceiveBeginPlay`
  (`parent.ReceiveBeginPlay`)
  (bind _returnvalue (`KismetMaterialLibrary.CreateDynamicMaterialInstance` "/Game/LandSpaceContent/Bunker/Materials/M_emisisve_Inst.M_emisisve_Inst"))
  (bind _output_get (set `self.Material` _returnvalue))
  (`PrimitiveComponent.SetMaterial` (`self.SM_lamp_02`) 1 _output_get)
  (`self.ShowNiagaraxiajian` 0.0)
  (bind _asbp_game_mode_1 (cast `/Game/ALocalContent/Blueprint/BP_GameMode1` (`GameplayStatics.GetGameMode`)))
  (set `self.As BP Game Mode 1` _asbp_game_mode_1)
  (add `/Game/ALocalContent/Blueprint/BP_GameMode1.OnDispatchLevel1PreStart` _asbp_game_mode_1 (delegate `OnDispatchLevel1PreStart_Event_0`)))

(event `OnDispatchLevel1PreStart_Event_0`
  (`self.OpenDoor`))

(event `StartTeleport`
  (params (Level :type Integer))
  (bind _audio (`self.Audio`))
  (bind _audio_2 (`self.Audio`))
  (bind _output_get (set `self.CurrentLevel` Level))
  (bind _output_get_2 (set `self.IsTop` (> _output_get (`self.lastLevel`))))
  (`LightComponent.SetIntensity` (`self.PointLight`) 3000.0)
  (`MaterialInstanceDynamic.SetVectorParameterValue` (`self.Material`) "color" (`self.Open`))
  (`self.ShowNiagaraxiajian` 1.5 _output_get_2)
  (`self.ShowElevatorNumber`)
  (`/Game/ALocalContent/Blueprint/BP_GameMode1.OnDispatchLevelMoveState` (`self.As BP Game Mode 1`) true _output_get)
  (if (`self.OpenDoorState`)
    (`self.CloseDoor`)
    (`ActorComponent.SetActive` _audio_2 true true)
    (`AudioComponent.SetSound` _audio_2 "/Game/LocalContent/Sound/ElevatorClose.ElevatorClose")
    (`AudioComponent.Play` _audio_2 0.0)
    (`KismetSystemLibrary.Delay` 3.7))
  (set `self.Start` true)
  (goto _label :!via `Reset`))

(event `CloseDoor`
  (bind _sk_liftboxdoor (`self.Sk_LiftBoxDoor`))
  (set `self.OpenDoorState` false)
  (bind _output_get (set `self.SpeedPosition` (`SkeletalMeshComponent.GetPosition` _sk_liftboxdoor)))
  (`SkeletalMeshComponent.SetAnimation` _sk_liftboxdoor "/Game/LandSpaceContent/Anim/LeftBox/Anim_LeftBox_Close.Anim_LeftBox_Close")
  (`SkeletalMeshComponent.SetPosition` _sk_liftboxdoor _output_get true)
  (`SkeletalMeshComponent.Play` _sk_liftboxdoor false))

(event `OpenDoor`
  (bind _sk_liftboxdoor (`self.Sk_LiftBoxDoor`))
  (set `self.OpenDoorState` true)
  (bind _output_get (set `self.SpeedPosition` (`SkeletalMeshComponent.GetPosition` _sk_liftboxdoor)))
  (`SkeletalMeshComponent.SetAnimation` _sk_liftboxdoor "/Game/LandSpaceContent/Anim/LeftBox/Anim_LeftBox_open.Anim_LeftBox_open")
  (`SkeletalMeshComponent.SetPosition` _sk_liftboxdoor _output_get true)
  (`SkeletalMeshComponent.Play` _sk_liftboxdoor false))

(event `ShowNiagaraxiajian`
  (params (InValue :type "Float (double-precision)") (IsTop :type Boolean))
  (bind _niagara (`self.Niagara`))
  (bind _niagara_2 (`self.Niagara`))
  (bind (_relativelocation_x _relativelocation_y) (`KismetMathLibrary.BreakVector` (`SceneComponent.RelativeLocation` _niagara_2)))
  (`NiagaraComponent.SetAsset` _niagara (select `bool` IsTop :`false` "/Game/LocalContent/FX/xiajian/NE_jt_System_Down.NE_jt_System_Down" :`true` "/Game/LocalContent/FX/xiajian/NE_jt_System_Top.NE_jt_System_Top" :!type "NiagaraSystem Object Reference"))
  (`SceneComponent.K2_SetRelativeLocation` _niagara_2 (`KismetMathLibrary.MakeVector` _relativelocation_x _relativelocation_y (`KismetMathLibrary.SelectFloat` 135.0 147.0 IsTop)) false false)
  (`NiagaraComponent.SetVariableFloat` _niagara "User.Rate" InValue))

(event `self.ReceiveTick`
  (params (DeltaSeconds :type "Float (single-precision)"))
  (bind _audio (`self.Audio`))
  (bind _levellocations (`self.LevelLocations`))
  (bind (_output_x _output_y _output_z) (`KismetMathLibrary.BreakVector` (`|GetArrayItem` _levellocations (`self.lastLevel`))))
  (bind _z (.z (`|GetArrayItem` _levellocations (`self.CurrentLevel`))))
  (bind _returnvalue (`KismetMathLibrary.FInterpTo_Constant` (.z (`self.K2_GetActorLocation`)) _z DeltaSeconds 100.0))
  (if (`self.Start`)
    (`self.K2_SetActorLocation` (`KismetMathLibrary.MakeVector` (.x (`self.K2_GetActorLocation`)) (.y (`self.K2_GetActorLocation`)) _returnvalue))
    (`self.ShowElevatorNumber`)
    (`|ExecutionSequence`
      (:`then_0`
        (if (> (/ (`KismetMathLibrary.Abs` (- _returnvalue _output_z)) (`KismetMathLibrary.Abs` (- _z _output_z))) 0.8)
          (`/Engine/EditorBlueprintResources/StandardMacros.DoOnce` false :!label _label
            (:`Completed`
              (`ActorComponent.SetActive` _audio true true)
              (`AudioComponent.SetSound` _audio "/Game/LocalContent/Sound/DT.DT")
              (`AudioComponent.Play` _audio 0.0)))))
      (:`then_1`
        (if (select `bool` (`self.IsTop`) :`false` (<= _returnvalue _z) :`true` (>= _returnvalue _z))
          (set `self.Start` false)
          (`self.ShowNiagaraxiajian` 0.0)
          (`self.OpenDoor`)
          (set `self.lastLevel` (`self.CurrentLevel`))
          (`/Game/ALocalContent/Blueprint/BP_GameMode1.OnDispatchLevelMoveState` (`self.As BP Game Mode 1`) false 0))))))

(event `ShowElevatorNumber`
  (bind _array_index (`self.Array Index`))
  (for (_array_element _array_index_2) (`self.LevelLocations`)
    (if (> (+ (.z (`self.K2_GetActorLocation`)) 50.0) (.z _array_element))
      (set `self.Array Index` _array_index_2)))
  (`StaticMeshComponent.SetStaticMesh` (`self.Number`) (select `int` _array_index :`0` "/Game/LocalContent/Meshes/Word/one.one" :`1` "/Game/LocalContent/Meshes/Word/one.one" :`2` "/Game/LocalContent/Meshes/Word/two.two" :`3` "/Game/LocalContent/Meshes/Word/three.three" :`4` "/Game/LocalContent/Meshes/Word/four.four" :`5` "/Game/LocalContent/Meshes/Word/five.five" :!type "StaticMesh Object Reference"))
  (`/Game/ALocalContent/Blueprint/BP_GameMode1.OnDispatchLevelNumChange` (`self.As BP Game Mode 1`) _array_index))

(fn `GetLevelBottomActor`
  (params (Level :type Integer)))

(fn `UserConstructionScript`)