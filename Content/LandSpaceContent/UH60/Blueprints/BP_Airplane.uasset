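; BP_Airplane is an aircraft actor in the UH60 content folder that bobs gently up and down in place.
; Tick advances a phase angle by scaled delta time and adds half its sine to the actor's current Z, leaving X and Y unchanged.
; Because that offset accumulates every frame without delta scaling, the bob's amplitude depends on frame rate.
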(event `self.ReceiveTick`
  (params (DeltaSeconds :type "Float (single-precision)"))
  (bind (_returnvalue_x _returnvalue_y _returnvalue_z) (`KismetMathLibrary.BreakVector` (`self.K2_GetActorLocation`)))
  (bind _output_get (set `self.NewVar_0` (+ (* DeltaSeconds 100.0) (`self.NewVar_0`))))
  (`self.K2_SetActorLocation` (`KismetMathLibrary.MakeVector` _returnvalue_x _returnvalue_y (+ _returnvalue_z (/ (`KismetMathLibrary.DegSin` _output_get) 2.0)))))

(fn `UserConstructionScript`)