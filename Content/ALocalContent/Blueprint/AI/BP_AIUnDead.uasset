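; Zombie AI character that patrols or walks to a set destination on level start, and triggers player death when it attacks.
; Blackboard states drive alert, battle, timed return and level reset, with randomized move types and patrol points built from placed actors.
; SpMove zombies are focusable: clicking the body alerts them to the player.
; Their socketed item (a work badge) slows the zombie on focus, then timelines fly it to camera and into the player.
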(event `/MCAI/Base/AI_IF_AIToBP.NotifyExecuteAttack`
  (params (TaskObj :type "BTTask_BlueprintBase Object Reference"))
  (set `self.ShortAttackMontage` "/Game/ALocalContent/SkeletalMesh/Anim/Attack/Zombie_Atk_Arms_3_IPC_Montage.Zombie_Atk_Arms_3_IPC_Montage")
  (`parent.NotifyExecuteAttack` TaskObj)
  (bind _asbp_game_mode_1 (cast `/Game/ALocalContent/Blueprint/BP_GameMode1` (`GameplayStatics.GetGameMode`)))
  (`/Game/ALocalContent/Blueprint/BP_GameMode1.PlayerDead` _asbp_game_mode_1))

(event `/MCAI/Base/AI_IF_AIToBP.NotifyExecuteEnterBattle`
  (params (TaskObj :type "BTTask_BlueprintBase Object Reference"))
  (`self.SetBBCombatState` "NewEnumerator3"))

(event `OnAlert`
  (if (`self.bSpMove`)
    (if (`|EnumInequality` (`self.GetBBCombatState`) "NewEnumerator3")
      (`KismetSystemLibrary.K2_ClearAndInvalidateTimerHandle` (`self.ReturnHandle`))
      (`self.SetBBCombatState` "NewEnumerator5")
      (`self.SetBBTargetObj` (`GameplayStatics.GetPlayerPawn` 0))
      (`self.SetBBState` "NewEnumerator2"))))

(event `OnReturn`
  (bind _returnvalue (`KismetSystemLibrary.K2_SetTimerDelegate` (delegate `CustomEvent_1`) 5.0))
  (set `self.ReturnHandle` _returnvalue))

(event `CustomEvent_1`
  (`self.SetBBCombatState` "NewEnumerator2")
  (`self.SetBBState` "NewEnumerator2"))

(event `self.ReceiveBeginPlay`
  (`self.InitMoveType`)
  (`self.InitPatroll`)
  (`self.InitAvandenMesh`)
  (if (`self.bUseAvandenMove`)
    (`parent.ReceiveBeginPlay`)
    (`KismetSystemLibrary.Delay` (`self.DelayMove`))
    (`self.OnStartTreeBase`)
    (if (`self.bSpMove`)
      (bind _asbp_game_mode_1 (cast `/Game/ALocalContent/Blueprint/BP_GameMode1` (`GameplayStatics.GetGameMode`)))
      (add `/Game/ALocalContent/Blueprint/BP_GameMode1.OnLevelReset` _asbp_game_mode_1 (delegate `OnLevelReset_Event_0`)))
    (else
      (bind _asbp_game_mode_1_2 (cast `/Game/ALocalContent/Blueprint/BP_GameMode1` (`GameplayStatics.GetGameMode`)))
      (add `/Game/ALocalContent/Blueprint/BP_GameMode1.OnDispatchLevel1Start` _asbp_game_mode_1_2 (delegate `CustomEvent_0`)))))

(event `OnLevelReset_Event_0`
  (bind _returnvalue (`SkeletalMeshComponent.GetAnimInstance` (`self.Mesh`)))
  (if (`|EnumEquality` (`self.GetBBCombatState`) "NewEnumerator3")
    (`KismetSystemLibrary.K2_ClearAndInvalidateTimerHandle` (`self.ReturnHandle`))
    (`AnimInstance.Montage_Stop` _returnvalue 0.0 (`AnimInstance.GetCurrentActiveMontage` _returnvalue))
    (`BTTask_BlueprintBase.FinishExecute` (`self.CurrentAttackCallTask`) true)
    (`self.SetBBCombatState` "NewEnumerator5")
    (`self.SetBBState` "NewEnumerator0")
    (`self.SetBBTargetObj` null)
    (`self.SetBBCombatState` "NewEnumerator2")
    (`self.SetBBState` "NewEnumerator2")))

(event `CustomEvent_0`
  (`KismetSystemLibrary.Delay` (`self.DelayMove`))
  (`|AIMoveTo` self (`self.NewVar_0`) null
    (:`then`
      (`self.OnStartMove`))
    (:`OnSuccess`
      (`self.OnEndMove` :!label _label))
    (:`OnFail`
      (goto _label))))

(event `/Game/ThirdPersonBP/Blueprints/BP_ClickInterface.OnClick`
  (params (ClickComponent :type "SceneComponent Object Reference"))
  (bind _returnvalue (`GameplayStatics.GetPlayerCameraManager` 0))
  (bind _equipobj (`self.EquipObj`))
  (bind _equipobj_2 (`self.EquipObj`))
  (bind _equipobj_3 (`self.EquipObj`))
  (bind _equipobj_4 (`self.EquipObj`))
  (if (== (`self.Mesh`) ClickComponent)
    (`self.OnAlert`)
    (`KismetSystemLibrary.PrintString` "发出噪音")
    (elif (== ClickComponent (`self.EquipObj`))
      (switch `/Game/ThirdPersonBP/Blueprints/EN_ClickState` (`self.E_ClickState`)
        (:`NewEnumerator1`
          (set `self.E_ClickState` "NewEnumerator0")
          (set `self.ObjectOriginLocation` (`SceneComponent.K2_GetComponentLocation` _equipobj_4))
          (`SceneComponent.K2_DetachFromComponent` _equipobj_4 "KeepWorld" "KeepWorld" "KeepWorld" true)
          (bind (_direction _newtrack_0) (`Timeline|Timeline_0` :!via `PlayFromStart`)
            (:`Update`
              (`SceneComponent.K2_SetWorldLocationAndRotation` _equipobj_3 (`KismetMathLibrary.VLerp` (`self.ObjectOriginLocation`) (+ (`PlayerCameraManager.GetCameraLocation` _returnvalue) (* (`self.GetActorForwardVector` _returnvalue) 40.0)) _newtrack_0) (`KismetMathLibrary.FindLookAtRotation` (`SceneComponent.K2_GetComponentLocation` _equipobj_3) (`PlayerCameraManager.GetCameraLocation` (`GameplayStatics.GetPlayerCameraManager` 0))) false false))))
        (:`NewEnumerator0`
          (set `self.ObjectOriginScale` (`SceneComponent.K2_GetComponentScale` _equipobj))
          (set `self.InspectionLocation` (`SceneComponent.K2_GetComponentLocation` _equipobj))
          (bind (_direction_2 _newtrack_0_2) (`Timeline|Timeline_2` :!via `PlayFromStart`)
            (:`Update`
              (`SceneComponent.SetWorldScale3D` _equipobj_2 (`KismetMathLibrary.VLerp` (`self.ObjectOriginScale`) (0.0 0.0 0.0) _newtrack_0_2))
              (`SceneComponent.K2_SetWorldLocation` _equipobj_2 (`KismetMathLibrary.VLerp` (`self.InspectionLocation`) (`KismetMathLibrary.MakeVector` (.x (`self.K2_GetActorLocation` (`GameplayStatics.GetPlayerPawn` 0))) (.y (`self.K2_GetActorLocation` (`GameplayStatics.GetPlayerPawn` 0))) (- (.z (`self.K2_GetActorLocation` (`GameplayStatics.GetPlayerPawn` 0))) 50.0)) _newtrack_0_2) false false))
            (:`Finished`
              (`KismetSystemLibrary.PrintString` "获取工作证"))))))))

(event `/Game/ThirdPersonBP/Blueprints/BP_ClickInterface.OnForce`
  (params (NewParam :type "SceneComponent Object Reference"))
  (bind _equipobj (`self.EquipObj`))
  (bind _mesh (`self.Mesh`))
  (if (== _mesh NewParam)
    (`PrimitiveComponent.SetRenderCustomDepth` _mesh true)
    (set `self.CustomTimeDilation` 1.0)
    (elif (== NewParam _equipobj)
      (`PrimitiveComponent.SetRenderCustomDepth` _equipobj true)
      (switch `/Game/ThirdPersonBP/Blueprints/EN_ClickState` (`self.E_ClickState`)
        (:`NewEnumerator1`
          (set `self.CustomTimeDilation` 0.05))))))

(event `/Game/ThirdPersonBP/Blueprints/BP_ClickInterface.OnUnForce`
  (params (NewParam :type "SceneComponent Object Reference"))
  (bind _mesh (`self.Mesh`))
  (bind _equipobj (`self.EquipObj`))
  (if (== _mesh NewParam)
    (`PrimitiveComponent.SetRenderCustomDepth` _mesh false)
    (set `self.CustomTimeDilation` 1.0)
    (elif (== NewParam _equipobj)
      (`PrimitiveComponent.SetRenderCustomDepth` _equipobj false)
      (set `self.CustomTimeDilation` 1.0))))

(fn `InitAvandenMesh`
  (if (`self.bSpMove`)
    (bind _returnvalue (`AddComponent|NODE_AddStaticMeshComponent-0` :`RelativeTransform` (`KismetMathLibrary.MakeTransform` (0.0 0.0 0.0))))
    (set `self.EquipObj` _returnvalue)
    (`SceneComponent.K2_AttachToComponent` _returnvalue (`self.Mesh`) "EquipSlot" "SnapToTarget" "SnapToTarget" "SnapToTarget" true)))

(fn `InitMoveType`
  (bind _premovetype (`self.PreMoveType`))
  (set `self.MoveType` (`KismetMathLibrary.SelectInt` (`KismetMathLibrary.RandomIntegerInRange` 1 4) _premovetype (== _premovetype 0))))

(fn `InitPatroll`
  (locals (LocationPatrolInfo :type "Array of /MCAI/Patrol/AI_ST_Patrol Structure"))
  ;[1 1 1] InPatrol
  (if (`self.bUseAvandenMove`)
    (for _array_element (`.PatrolPointParam_19_199292664A298B9CFB9775AABA3109C0` (break `/MCAI/Base/AI_ST_InitDefault` (`self.DefaultInfo`)))
      (bind (_movepoint _usedirection _pointlocation _pointdirection _arrivepointpose _earlyendtime _beforeanimdelaymintime _beforeanimdelaymaxtime _afteranimdelaymintime _afteranimdelaymaxtime) (break `/MCAI/Patrol/AI_ST_Patrol` _array_element))
      (`/Engine/EditorBlueprintResources/StandardMacros.IsValid` _movepoint
        (:`Is Valid`
          (`KismetArrayLibrary.Array_Add` (`local.LocationPatrolInfo`) (make `/MCAI/Patrol/AI_ST_Patrol` _movepoint _usedirection (`SceneComponent.K2_GetComponentLocation` (`/MCAI/Patrol/AI_Patrol_Path_Point.Point` _movepoint)) (`SceneComponent.K2_GetComponentRotation` (`/MCAI/Patrol/AI_Patrol_Path_Point.Arrow` _movepoint)) _arrivepointpose _earlyendtime _beforeanimdelaymintime _beforeanimdelaymaxtime _afteranimdelaymintime _afteranimdelaymaxtime)))))
    (setmembers `/MCAI/Base/AI_ST_InitDefault` :`StructRef` (`self.DefaultInfo`) :`PatrolPointParam` (`local.LocationPatrolInfo`))))

(fn `IsCanForce`
  (params (NewParam :type "SceneComponent Object Reference") (Distance :type "Float (double-precision)"))
  (returns (IsCan :type Boolean))
  (if (`self.bSpMove`)
    (if (== (`self.EquipObj`) NewParam)
      (switch `/Game/ThirdPersonBP/Blueprints/EN_ClickState` (`self.E_ClickState`)
        (:`NewEnumerator1`
          (return (< Distance 300.0)))
        (:`NewEnumerator0`
          (return true)))
      (else
        (return true)))
    (else
      (return false))))

(fn `OnEndMove`
  (set `self.MoveSpeedType` 0))

(fn `OnStartMove`
  (bind _premovespeedtype (`self.PreMoveSpeedType`))
  (set `self.MoveSpeedType` (`KismetMathLibrary.SelectInt` (`KismetMathLibrary.RandomIntegerInRange` 1 3) _premovespeedtype (== _premovespeedtype 0))))

(fn `UserConstructionScript`)