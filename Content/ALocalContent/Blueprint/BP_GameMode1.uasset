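; Game mode Blueprint that sequences the level 1 opening and the player's death and revive cycle.
; GameStart fires pre-start and start dispatchers on timed delays, then starts and later stops teleporting on the first BP_Elevator found.
; PlayerDead broadcasts death and animates the Die parameter in the Blood_Param collection through a timeline.
; When the timeline finishes, it broadcasts a level reset, waits, then clears the parameter and broadcasts revive.
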(event `self.ReceiveBeginPlay`)

(event `GameStart`
  (`KismetSystemLibrary.PrintString` "游戏开始")
  (`KismetSystemLibrary.Delay` 1.0)
  (`self.OnDispatchLevel1PreStart`)
  (`KismetSystemLibrary.Delay` 2.0)
  (`self.OnDispatchLevel1Start`)
  (`KismetSystemLibrary.Delay` 22.0)
  (bind _outactors (`GameplayStatics.GetAllActorsOfClass` "/Game/LandSpaceContent/BluePrint/BP_Elevator.BP_Elevator_C"))
  (bind _output (`|GetArrayItem` _outactors))
  (`/Game/LandSpaceContent/BluePrint/BP_Elevator.StartTeleport` _output 2)
  (`KismetSystemLibrary.Delay` 5.0)
  (`/Game/LandSpaceContent/BluePrint/BP_Elevator.StopTeleport` _output))

(event `PlayerDead`
  (`self.OnPlayerDead`)
  (bind (_direction _newtrack_0) (`Timeline|Timeline_0` :!via `PlayFromStart`)
    (:`Update`
      (`KismetMaterialLibrary.SetScalarParameterValue` "/Game/LocalContent/Other/Blood_Param.Blood_Param" "Die" _newtrack_0))
    (:`Finished`
      (`self.OnLevelReset`)
      (`KismetSystemLibrary.Delay` 5.0)
      (`self.PlayerRevive`))))

(event `PlayerRevive`
  (`KismetMaterialLibrary.SetScalarParameterValue` "/Game/LocalContent/Other/Blood_Param.Blood_Param" "Die")
  (`self.OnPlayerRevive`))

(fn `UserConstructionScript`)