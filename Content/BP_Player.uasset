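; BP_Player is a player actor that views the level through the first CineCameraActor found and tests mouse picking.
; Left click picks player controller 0 or 1 by viewport half, suggesting split screen, then line-traces the deprojected cursor on Visibility.
; Hits only draw a debug sphere; print and destroy nodes are disconnected.
; AI-facing getters for camp, damage, death, avoidance and pawn components return fixed or default values.
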(event `self.ReceiveBeginPlay`
  (bind _outactors (`GameplayStatics.GetAllActorsOfClass` "/Script/CinematicCamera.CineCameraActor"))
  (`PlayerController.SetViewTargetWithBlend` (`GameplayStatics.GetPlayerController` 0) (`|GetArrayItem` _outactors) 0.0 "VTBlend_Linear" 0.0 false))

(event `InputAction|LeftMouse`
  (params (Key :type "Key Structure"))
  (:`Pressed`
    (bind _returnvalue (`WidgetLayoutLibrary.GetMousePositionOnViewport`))
    (bind _output_get (set `self.PlayerIndex` (select `bool` (> (`KismetMathLibrary.BreakVector2D` _returnvalue) (/ (`KismetMathLibrary.BreakVector2D` (`WidgetLayoutLibrary.GetViewportSize`)) 2.0)) :`true` 1)))
    (bind (_worldlocation _worlddirection) (`PlayerController.DeprojectMousePositionToWorld` (`GameplayStatics.GetPlayerController` _output_get)))
    (bind (_outhit _returnvalue_2) (`KismetSystemLibrary.LineTraceSingle` :`Start` _worldlocation :`End` (+ (* _worlddirection 5000.0) _worldlocation) :`TraceChannel` "TraceTypeQuery1" :`DrawDebugType` "ForDuration"))
    (if _returnvalue_2
      (`KismetSystemLibrary.DrawDebugSphere` (`.Location` (`GameplayStatics.BreakHitResult` _outhit)) 50.0 12 (struct :`R` 1.0 :`B` 0.183144 :`A` 1.0) 2.0))))

(event `self.ReceiveTick`
  (params (DeltaSeconds :type "Float (single-precision)")))

(fn `GetAvoidGroup`
  (returns (AvoidGroup :type "NavAvoidanceMask Structure"))
  (return))

(fn `GetCampType`
  (returns (CampStruct :type "/MCAI/Base/AI_ST_InitCamp Structure"))
  (return (make `/MCAI/Base/AI_ST_InitCamp` "NewEnumerator0" "NewEnumerator2" "NewEnumerator0")))

(fn `GetDamageParam`
  (returns (DamageDirection :type "/MCAI/Direction/EN_3DDirection_Simple Enum"))
  (return "NewEnumerator0"))

(fn `GetIsDead`
  (returns (IsDead :type Boolean))
  (return false))

(fn `GetPawnComponent`
  (returns (MoveTargetActor :type "Actor Object Reference") (RootComponent :type "SceneComponent Object Reference"))
  (return self (`self.CapsuleComponent`)))

(fn `UserConstructionScript`)